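; Enemy actor that rotates to face the player's Arwing and fires lasers at it, and can be shot down.
; PawnSensing sightings aim it at a point offset along world X from the Arwing, then, after a delay, spawn an enemy laser at the mesh's Shot socket toward that point.
; Overlapping player lasers subtract damage from Life and are destroyed, while Tick destroys the enemy once Life runs out.
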(event OnSeePawn(PawnSensing)
  (params (Pawn :type Pawn%20Object%20Reference))
  (bind _asbp_arwing (Utilities|Casting|CastToBP_Arwing Pawn))
  (Utilities|FlowControl|Sequence
    (:then_0
      (Transformation|SetActorRotation (Math|Rotator|FindLookatRotation (Transformation|GetActorLocation) (Math|Vector|MakeVector (+ (.x (Transformation|GetActorLocation _asbp_arwing)) 1e+02) (.y (Transformation|GetActorLocation _asbp_arwing)) (.z (Transformation|GetActorLocation _asbp_arwing))))))
    (:then_1
      (Utilities|FlowControl|Delay 1.0)
      (bind _returnvalue (Game|SpawnActorfromClass "/Game/Blueprint/BP_LaserShorEnemi.BP_LaserShorEnemi_C" (Math|Transform|MakeTransform (Transformation|GetSocketLocation (Variables|Default|GetBandit_0_orange_metal) "Shot") (Math|Rotator|FindLookatRotation (Transformation|GetActorLocation) (Math|Vector|MakeVector (+ (.x (Transformation|GetActorLocation _asbp_arwing)) 1e+02) (.y (Transformation|GetActorLocation _asbp_arwing)) (.z (Transformation|GetActorLocation _asbp_arwing)))) "10.000000,10.000000,10.000000") "Undefined" 0 0))
      (Class|ProjectileMovementComponent|MoveInterpolationTarget (Variables|/Game/Blueprint/BP_LaserShorEnemi.BP_LaserShorEnemi_C|GetProjectileMovement _returnvalue) (Math|Vector|MakeVector (+ (.x (Transformation|GetActorLocation _asbp_arwing)) 1e+02) (.y (Transformation|GetActorLocation _asbp_arwing)) (.z (Transformation|GetActorLocation _asbp_arwing))) (Math|Rotator|FindLookatRotation (Transformation|GetActorLocation) (Math|Vector|MakeVector (+ (.x (Transformation|GetActorLocation _asbp_arwing)) 1e+02) (.y (Transformation|GetActorLocation _asbp_arwing)) (.z (Transformation|GetActorLocation _asbp_arwing))))))))

(event EventTick
  (params (DeltaSeconds :type Float%20%28single-precision%29))
  (if (<= (Variables|Default|GetLife) 0.0)
    (Actor|DestroyActor)))

(event Collision|EventActorBeginOverlap
  (params (OtherActor :type Actor%20Object%20Reference))
  (bind _asbp_laser_shor (Utilities|Casting|CastToBP_LaserShor OtherActor))
  (Variables|Default|SetLife (- (Variables|Default|GetLife) (Variables|/Game/Blueprint/BP_LaserShor.BP_LaserShor_C|GetDamage _asbp_laser_shor)))
  (Actor|DestroyActor _asbp_laser_shor))

(fn ConstructionScript)
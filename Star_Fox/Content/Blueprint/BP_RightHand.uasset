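; BP_RightHand is a destructible right-hand actor with its own Life value that takes damage from laser shots.
; On overlap with a BP_LaserShor, it subtracts that shot's Damage from Life and destroys the shot.
; Each Tick loops over all BP_Adross actors but tests only its own Life, destroying itself at zero or below if any BP_Adross exists.
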(event EventBeginPlay)

(event Collision|EventActorBeginOverlap
  (params (OtherActor :type Actor%20Object%20Reference))
  (bind _asbp_laser_shor (Utilities|Casting|CastToBP_LaserShor OtherActor))
  (Variables|Default|SetLife (- (Variables|Default|GetLife) (Variables|/Game/Blueprint/BP_LaserShor.BP_LaserShor_C|GetDamage _asbp_laser_shor)))
  (Actor|DestroyActor _asbp_laser_shor))

(event EventTick
  (params (DeltaSeconds :type Float%20%28single-precision%29))
  (bind _outactors (Actor|GetAllActorsOfClass "/Game/Blueprint/BP_Adross.BP_Adross_C"))
  (for _array_element _outactors
    (if (<= (Variables|Default|GetLife) 0.0)
      (Actor|DestroyActor))))

(fn ConstructionScript)
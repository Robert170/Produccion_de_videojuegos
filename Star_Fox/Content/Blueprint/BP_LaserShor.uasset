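; Laser shot actor, judging by its name, that gains damage when it overlaps upgrade actors.
; Each overlap with a BP_Upgrade raises its Level by one.
; Reaching the second and third levels sets Damage to increasing multiples of OriginDam, and higher levels leave Damage unchanged.
; The Blueprint holds no movement or damage-dealing logic.
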(event EventBeginPlay)

(event Collision|EventActorBeginOverlap
  (params (OtherActor :type Actor%20Object%20Reference))
  (Utilities|Casting|CastToBP_Upgrade OtherActor)
  (Variables|Default|SetLevel (+ (Variables|Default|GetLevel) 1.0))
  (if (== (Variables|Default|GetLevel) 2.0)
    (Variables|Default|SetDamage (* (Variables|Default|GetOrigin_Dam) 1.5))
    (elif (== (Variables|Default|GetLevel) 3.0)
      (Variables|Default|SetDamage (* (Variables|Default|GetOrigin_Dam) 2.0)))))

(event EventTick
  (params (DeltaSeconds :type Float%20%28single-precision%29)))

(fn ConstructionScript)
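; BP_LeftHand is a destructible hand, apparently part of the BP_Adross enemy, that travels along a spline.
; Overlapping BP_LaserShor shots subtract their damage from Life and are destroyed.
; Tick loops over BP_Adross actors, destroying the hand at zero Life or driving a timeline that moves and rotates Scene along Spline.
; A SplineFinish flag switches between delayed play and reverse; the Adross Life check is unconnected.
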(event EventBeginPlay)

(event Collision|EventActorBeginOverlap
  (params (OtherActor :type Actor%20Object%20Reference))
  (bind _asbp_laser_shor (Utilities|Casting|CastToBP_LaserShor OtherActor))
  (Variables|Default|SetLife (- (Variables|Default|GetLife) (Variables|/Game/Blueprint/BP_LaserShor.BP_LaserShor_C|GetDamage _asbp_laser_shor)))
  (Actor|DestroyActor _asbp_laser_shor))

(event EventTick
  (params (DeltaSeconds :type Float%20%28single-precision%29))
  (bind _scene (Variables|Default|GetScene))
  (bind _spline (Variables|Default|GetSpline))
  (bind _outactors (Actor|GetAllActorsOfClass "/Game/Blueprint/BP_Adross.BP_Adross_C"))
  (for _array_element _outactors
    (if (<= (Variables|Default|GetLife) 0.0)
      (Actor|DestroyActor)
      (elif (Math|Boolean|Equal(Boolean) (Variables|Default|GetSpline_finish) false)
        (Utilities|FlowControl|Delay 7.0)
        (bind _traveldistance (Timeline|Timeline_0 Play)
          (:Update
            (Transformation|SetWorldLocation _scene (Spline|GetLocationatDistanceAlongSpline _spline (* _traveldistance (Spline|GetSplineLength (Variables|Default|GetSpline))) "World") false false)
            (Transformation|SetRelativeRotation _scene (Spline|GetRotationatDistanceAlongSpline _spline (* _traveldistance (Spline|GetSplineLength (Variables|Default|GetSpline))) "Local") false false)
            (Variables|Default|SetSpline_finish true)))
        (else
          (Variables|Default|SetSpline_finish false)
          (Timeline|Timeline_0 Reverse))))))

(fn ConstructionScript)
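; Player Arwing ship for a Star Fox-style rail shooter, with health, lives, boost gas and pickups.
; Tick advances the Sphere along X, moves the Body within box bounds and runs barrel rolls, which block enemy lasers.
; Brake plus Down plays a timeline-driven spline somersault that suspends steering.
; Keys drive boost, brake, camera toggle, bombs and lasers, which upgrade to twin shots or charge through a hold timer.
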(event EventBeginPlay)

(event Collision|EventActorBeginOverlap
  (params (OtherActor :type Actor%20Object%20Reference))
  ;[1 1 1] Take_Objects
  (bind _asbp_silver_ring (Utilities|Casting|CastToBP_Silver_ring OtherActor)
    (:then
      (if (!= (Variables|Default|GetHealt) (Variables|Default|GetActual_healt))
        (Variables|Default|SetHealt (+ (Variables|Default|GetHealt) 1e+01))
        (Audio|SpawnSoundatLocation "/Game/Sounds/Laser_objects/bomb_pickup.bomb_pickup" "0, 0, 0" "0, 0, 0" 1.0 1.0 0.0 0 0)
        (Actor|DestroyActor _asbp_silver_ring)))
    (:CastFailed
      (bind _asbp_bbomb (Utilities|Casting|CastToBP_Bbomb OtherActor)
        (:then
          (Variables|Default|SetB_Bombs (+ (Variables|Default|GetB_Bombs) 1))
          (Audio|SpawnSoundatLocation "/Game/Sounds/Laser_objects/bomb_pickup.bomb_pickup" "0, 0, 0" "0, 0, 0" 1.0 1.0 0.0 0 0)
          (Actor|DestroyActor _asbp_bbomb))
        (:CastFailed
          (bind _asbp_upgrade (Utilities|Casting|CastToBP_Upgrade OtherActor)
            (:then
              (Variables|Default|SetLevel_Shot (+ (Variables|Default|GetLevel_Shot) 1))
              (Audio|SpawnSoundatLocation "/Game/Sounds/Laser_objects/bomb_pickup.bomb_pickup" "0, 0, 0" "0, 0, 0" 1.0 1.0 0.0 0 0)
              (Actor|DestroyActor _asbp_upgrade))
            (:CastFailed
              (Utilities|Casting|CastToBP_Enemi OtherActor
                (:then
                  (Variables|Default|SetHealt (- (Variables|Default|GetHealt) 5e+01)))
                (:CastFailed
                  (bind _asbp_laser_shor_enemi (Utilities|Casting|CastToBP_LaserShorEnemi OtherActor)
                    (:then
                      (if (Math|Boolean|Equal(Boolean) (Variables|Default|GetBarrerrol) false)
                        (Variables|Default|SetHealt (- (Variables|Default|GetHealt) (Variables|/Game/Blueprint/BP_LaserShorEnemi.BP_LaserShorEnemi_C|GetDamage _asbp_laser_shor_enemi)))))
                    (:CastFailed
                      (Utilities|Casting|CastToBP_Stop OtherActor)
                      (Variables|Default|Setvelocidad 0.0)
                      (Variables|Default|SetV 0.0)
                      (Variables|Default|SetAceleracion 0.0)
                      (Variables|Default|SetFreno 0.0))))))))))))

(event EventTick
  (params (DeltaSeconds :type Float%20%28single-precision%29))
  (bind _sphere (Variables|Default|GetSphere))
  (bind _spline (Variables|Default|GetSpline))
  (bind _returnvalue (Transformation|GetWorldLocation _sphere))
  ;[1 1 1] Movement Front
  (if (< (Variables|Default|GetHealt) (/ (Variables|Default|GetHealt) 2.0))
    (Audio|SpawnSoundatLocation "/Game/Sounds/Laser_objects/damage_alert_heavy.damage_alert_heavy" "0, 0, 0" "0, 0, 0" 1.0 1.0 0.0 0 0))
  (if (<= (Variables|Default|GetHealt) 0.0)
    (CallFunction|LoseLife)
    (elif (and (Math|Boolean|Equal(Boolean) (Variables|Default|GetM_D) true) (Math|Boolean|Equal(Boolean) (Variables|Default|GetC_S) true))
      (Variables|Default|SetGAS (- (Variables|Default|GetGAS) 1.0))
      (if (Math|Boolean|Equal(Boolean) (Variables|Default|GetMove_360) false)
        (Variables|Default|SetMove_360 true)
        (bind _traveldistance (Timeline|360 PlayFromStart)
          (:Update
            (Transformation|SetWorldLocation (Variables|Default|Getdummy) (Spline|GetLocationatDistanceAlongSpline _spline (* _traveldistance (Spline|GetSplineLength (Variables|Default|GetSpline))) "World") false false)
            (Transformation|SetRelativeRotation (Variables|Default|Getdummy) (Spline|GetRotationatDistanceAlongSpline _spline (* _traveldistance (Spline|GetSplineLength (Variables|Default|GetSpline))) "Local") false false))
          (:Finished
            (Variables|Default|SetM_D false)
            (Variables|Default|SetC_S false)
            (Variables|Default|SetMove_360 false)
            (Transformation|AddLocalOffset (Variables|Default|GetBody) (* (stale _returnvalue_2) DeltaSeconds) false false :!label _label)
            (Transformation|SetWorldLocation _sphere (Math|Vector|MakeVector (+ (.x _returnvalue) (Variables|Default|Getvelocidad)) (.y _returnvalue) (.z _returnvalue)) false false)
            (if (Math|Boolean|ORBoolean (Math|Boolean|Equal(Boolean) (Variables|Default|GetC_A) true) (Math|Boolean|Equal(Boolean) (Variables|Default|GetC_S) true) false)
              (if (== (Variables|Default|GetGAS) 0.0)
                (Variables|Default|SetC_A false)
                (Variables|Default|SetC_S false)
                (Variables|Default|Setvelocidad (Variables|Default|GetVel_mov))
                (else
                  (Variables|Default|SetGAS (- (Variables|Default|GetGAS) 1.0))))
              (elif (< (Variables|Default|GetGAS) (Variables|Default|GetActual_Gas))
                (Variables|Default|SetGAS (+ (Variables|Default|GetGAS) 1.0))))
            (if (Math|Boolean|Equal(Boolean) (Variables|Default|GetBarrerrol) true)
              (CallFunction|Barreroll))))
        (else
          (Timeline|360 PlayFromStart)))
      (elif (not (Math|Boolean|Equal(Boolean) (Variables|Default|GetMove_360) true))
        (bind _returnvalue_2 (Class|Pawn|ConsumeMovementInputVector))
        (goto _label)))))

(event Input|AxisEvents|InputAxisArwing_Move_D
  (params (AxisValue :type Float%20%28single-precision%29))
  ;[1 1 1] Movement U, D, R, L
  (if (not (and (Math|Boolean|Equal(Boolean) (Variables|Default|GetM_D) true) (Math|Boolean|Equal(Boolean) (Variables|Default|GetC_S) true)))
    (if (> (.z (Transformation|GetWorldLocation (Variables|Default|GetArwing_Body))) (.z (Transformation|GetWorldLocation (Variables|Default|GetBox_down))))
      (Pawn|Input|AddMovementInput (Math|Vector|VectorUp) (* AxisValue (Variables|Default|GetVel_mov)) false))))

(event Input|AxisEvents|InputAxisArwing_Move_U
  (params (AxisValue :type Float%20%28single-precision%29))
  ;[1 1 1] Movement U, D, R, L
  (if (not (and (Math|Boolean|Equal(Boolean) (Variables|Default|GetM_D) true) (Math|Boolean|Equal(Boolean) (Variables|Default|GetC_S) true)))
    (if (< (.z (Transformation|GetWorldLocation (Variables|Default|GetArwing_Body))) (.z (Transformation|GetWorldLocation (Variables|Default|GetBox_up))))
      (Pawn|Input|AddMovementInput (Math|Vector|VectorUp) (* AxisValue (Variables|Default|GetVel_mov)) false))))

(event Input|AxisEvents|InputAxisArwing_Move_R
  (params (AxisValue :type Float%20%28single-precision%29))
  ;[1 1 1] Movement U, D, R, L
  (if (not (and (Math|Boolean|Equal(Boolean) (Variables|Default|GetM_D) true) (Math|Boolean|Equal(Boolean) (Variables|Default|GetC_S) true)))
    (if (< (.y (Transformation|GetWorldLocation (Variables|Default|GetArwing_Body))) (.y (Transformation|GetWorldLocation (Variables|Default|GetBox_Rigth))))
      (Pawn|Input|AddMovementInput (Class|KismetMathLibrary|VectorRight) (* AxisValue (Variables|Default|GetVel_mov)) false))))

(event Input|AxisEvents|InputAxisArwing_Move_L
  (params (AxisValue :type Float%20%28single-precision%29))
  ;[1 1 1] Movement U, D, R, L
  (if (not (and (Math|Boolean|Equal(Boolean) (Variables|Default|GetM_D) true) (Math|Boolean|Equal(Boolean) (Variables|Default|GetC_S) true)))
    (if (not (< (.y (Transformation|GetWorldLocation (Variables|Default|GetArwing_Body))) (.y (Transformation|GetWorldLocation (Variables|Default|GetBox_Left)))))
      (Pawn|Input|AddMovementInput (Class|KismetMathLibrary|VectorRight) (* AxisValue (Variables|Default|GetVel_mov)) false))))

(event Input|KeyboardEvents|A
  (params (Key :type Key%20Structure))
  ;[1 1 1] C Buttons
  (:Pressed
    (Variables|Default|SetC_A true)
    (Audio|SpawnSoundatLocation "/Game/Sounds/Laser_objects/boost.boost" "0, 0, 0" "0, 0, 0" 1.0 1.0 0.0 0 0)
    (Variables|Default|Setvelocidad (Variables|Default|GetAceleracion)))
  (:Released
    (Variables|Default|SetC_A false)
    (Variables|Default|Setvelocidad 5e+01)))

(event Input|KeyboardEvents|S
  (params (Key :type Key%20Structure))
  ;[1 1 1] C Buttons
  (:Pressed
    (Variables|Default|SetC_S true)
    (Audio|SpawnSoundatLocation "/Game/Sounds/Laser_objects/break.break" "0, 0, 0" "0, 0, 0" 1.0 1.0 0.0 0 0)
    (Variables|Default|Setvelocidad (Variables|Default|GetFreno)))
  (:Released
    (Variables|Default|SetC_S false)
    (Variables|Default|Setvelocidad (Variables|Default|GetVel_mov))))

(event Input|KeyboardEvents|X
  (params (Key :type Key%20Structure))
  ;[1 1 1] Shots
  (:Pressed
    (Utilities|Time|SetTimerbyFunctionName 0 "Time_Button_press" 1.0 true)
    (Variables|Default|SetX_Press true)
    (if (> (Variables|Default|GetLevel_Shot) 1)
      (Audio|SpawnSoundatLocation "/Game/Sounds/Laser_objects/arwing_double_laser_one_shot.arwing_double_laser_one_shot" "0, 0, 0" "0, 0, 0" 1.0 1.0 0.0 0 0)
      (CallFunction|ShotLevel2or3)
      (else
        (Audio|SpawnSoundatLocation "/Game/Sounds/Laser_objects/arwing_single_laser_one_shot.arwing_single_laser_one_shot" "0, 0, 0" "0, 0, 0" 1.0 1.0 0.0 0 0)
        (CallFunction|ShotLevel1))))
  (:Released
    (Variables|Default|SetX_Press false)
    (if (>= (Variables|Default|GetTime_press_button) 3)
      (Variables|Default|SetTime_press_button 0)
      (CallFunction|ShotCharge))))

(event Input|KeyboardEvents|C
  (params (Key :type Key%20Structure))
  ;[1 1 1] Shots
  (:Pressed
    (if (> (Variables|Default|GetB_Bombs) 0)
      (bind _returnvalue (Game|SpawnActorfromClass "/Game/Blueprint/BP_Bbomb_shot.BP_Bbomb_shot_C" (Math|Transform|MakeTransform (Transformation|GetSocketLocation (Variables|Default|GetArwing_Body) "Shot_Laser_Socket") "0, 0, 0" "5.000000,5.000000,5.000000") "Undefined" 0 0))
      (bind _output_get (Variables|/Script/Engine.ProjectileMovementComponent|SetInitialSpeed (Variables|/Game/Blueprint/BP_Bbomb_shot.BP_Bbomb_shot_C|GetProjectileMovement _returnvalue) (* (Variables|Default|GetShot_Vel) 1e+02)))
      (bind _output_get_2 (Variables|/Script/Engine.ProjectileMovementComponent|SetMaxSpeed (Variables|/Game/Blueprint/BP_Bbomb_shot.BP_Bbomb_shot_C|GetProjectileMovement _returnvalue) _output_get))
      (Variables|/Script/Engine.MovementComponent|SetVelocity (Variables|/Game/Blueprint/BP_Bbomb_shot.BP_Bbomb_shot_C|GetProjectileMovement _returnvalue) (Math|Vector|MakeVector _output_get_2 0.0 0.0))
      (Variables|Default|SetB_Bombs (- (Variables|Default|GetB_Bombs) 1)))))

(event Input|KeyboardEvents|Down
  (params (Key :type Key%20Structure))
  ;[1 1 1] C Buttons
  (:Pressed
    (Variables|Default|SetM_D true))
  (:Released
    (if (not (Math|Boolean|Equal(Boolean) (Variables|Default|GetMove_360) true))
      (Variables|Default|SetM_D false))))

(event Input|KeyboardEvents|D
  (params (Key :type Key%20Structure))
  ;[1 1 1] C Buttons
  (:Pressed
    (Variables|Default|SetC_D true))
  (:Released
    (if (not (Math|Boolean|Equal(Boolean) (Variables|Default|GetMove_360) true))
      (Variables|Default|SetC_D false))))

(event Input|KeyboardEvents|W
  (params (Key :type Key%20Structure))
  ;[1 1 1] C Buttons
  (:Pressed
    (Utilities|FlowControl|FlipFlop
      (:A
        (Components|Activation|Deactivate (Variables|Default|GetMain_Camera))
        (Components|Activation|SetActive (Variables|Default|GetFirst_Person_camera) true false)
        (Variables|Default|SetVel_mov 1e+04))
      (:B
        (Components|Activation|SetActive (Variables|Default|GetMain_Camera) true false)
        (Variables|Default|SetVel_mov 2e+02)))))

(event Input|KeyboardEvents|SpaceBar
  (params (Key :type Key%20Structure))
  ;[1 1 1] Barreroll
  (:Pressed
    (Math|Integer|IncrementInt (Variables|Default|GetDo_Barreroll)
      (:%20%20
        (if (== (Variables|Default|GetDo_Barreroll) 2)
          (Variables|Default|SetBarrerrol true))))))

(event Input|KeyboardEvents|Y
  (params (Key :type Key%20Structure))
  (:Pressed
    (Variables|Default|SetHealt (- (Variables|Default|GetHealt) 1e+01))))

(event Input|KeyboardEvents|Right
  (params (Key :type Key%20Structure))
  ;[1 1 1] Move Buttons
  (:Pressed
    (Variables|Default|SetRot_Rigth true))
  (:Released
    (Variables|Default|SetRot_Rigth false)))

(event Input|KeyboardEvents|U
  (params (Key :type Key%20Structure))
  (:Pressed
    (Variables|Default|SetHealt (+ (Variables|Default|GetHealt) 1e+01))))

(event Input|KeyboardEvents|E
  (params (Key :type Key%20Structure))
  ;[1 1 1] Move Buttons
  (:Pressed
    (Variables|Default|SetInclinacion_D true))
  (:Released
    (Variables|Default|SetInclinacion_D false)))

(event Input|KeyboardEvents|Q
  (params (Key :type Key%20Structure))
  ;[1 1 1] Move Buttons
  (:Pressed
    (Variables|Default|SetInclinacion_I true))
  (:Released
    (Variables|Default|SetInclinacion_I false)))

(fn ConstructionScript)

(fn G360)

(fn ShotLevel1
  (bind _returnvalue (Game|SpawnActorfromClass "/Game/Blueprint/BP_LaserShor.BP_LaserShor_C" (Math|Transform|MakeTransform (Transformation|GetSocketLocation (Variables|Default|GetArwing_Body) "Shot_Laser_Socket") "0, 0, 0" "2.000000,2.000000,2.000000") "Undefined" 0 0))
  (bind _output_get (Variables|/Script/Engine.ProjectileMovementComponent|SetInitialSpeed (Variables|/Game/Blueprint/BP_LaserShor.BP_LaserShor_C|GetProjectileMovement _returnvalue) (* (Variables|Default|GetShot_Vel) 1e+02)))
  (bind _output_get_2 (Variables|/Script/Engine.ProjectileMovementComponent|SetMaxSpeed (Variables|/Game/Blueprint/BP_LaserShor.BP_LaserShor_C|GetProjectileMovement _returnvalue) _output_get))
  (Variables|/Script/Engine.MovementComponent|SetVelocity (Variables|/Game/Blueprint/BP_LaserShor.BP_LaserShor_C|GetProjectileMovement _returnvalue) (Math|Vector|MakeVector _output_get_2 0.0 0.0)))

(fn ShotLevel2or3
  (bind _returnvalue (Game|SpawnActorfromClass "/Game/Blueprint/BP_LaserShor.BP_LaserShor_C" (Math|Transform|MakeTransform (Transformation|GetSocketLocation (Variables|Default|GetArwing_Mesh8_skp743B1_Model) "Shot_socket_l2") "0, 0, 0" "2.000000,2.000000,2.000000") "Undefined" 0 0))
  (bind _output_get (Variables|/Script/Engine.ProjectileMovementComponent|SetInitialSpeed (Variables|/Game/Blueprint/BP_LaserShor.BP_LaserShor_C|GetProjectileMovement _returnvalue) (* (Variables|Default|GetShot_Vel) 1e+02)))
  (bind _output_get_2 (Variables|/Script/Engine.ProjectileMovementComponent|SetMaxSpeed (Variables|/Game/Blueprint/BP_LaserShor.BP_LaserShor_C|GetProjectileMovement _returnvalue) _output_get))
  (Variables|/Script/Engine.MovementComponent|SetVelocity (Variables|/Game/Blueprint/BP_LaserShor.BP_LaserShor_C|GetProjectileMovement _returnvalue) (Math|Vector|MakeVector _output_get_2 0.0 0.0))
  (bind _returnvalue_2 (Game|SpawnActorfromClass "/Game/Blueprint/BP_LaserShor.BP_LaserShor_C" (Math|Transform|MakeTransform (Transformation|GetSocketLocation (Variables|Default|GetArwing_Mesh3_skp743B1_Model) "Socket_Shot_L2") "0, 0, 0" "2.000000,2.000000,2.000000") "Undefined" 0 0))
  (bind _output_get_3 (Variables|/Script/Engine.ProjectileMovementComponent|SetInitialSpeed (Variables|/Game/Blueprint/BP_LaserShor.BP_LaserShor_C|GetProjectileMovement _returnvalue_2) (* (Variables|Default|GetShot_Vel) 1e+02)))
  (bind _output_get_4 (Variables|/Script/Engine.ProjectileMovementComponent|SetMaxSpeed (Variables|/Game/Blueprint/BP_LaserShor.BP_LaserShor_C|GetProjectileMovement _returnvalue_2) _output_get_3))
  (Variables|/Script/Engine.MovementComponent|SetVelocity (Variables|/Game/Blueprint/BP_LaserShor.BP_LaserShor_C|GetProjectileMovement _returnvalue_2) (Math|Vector|MakeVector _output_get_4 0.0 0.0)))

(fn ShotCharge
  (bind _returnvalue (Game|SpawnActorfromClass "/Game/Blueprint/BP_LaserShor.BP_LaserShor_C" (Math|Transform|MakeTransform (Transformation|GetSocketLocation (Variables|Default|GetArwing_Body) "Shot_Laser_Socket") "0, 0, 0" "20.000000,20.000000,20.000000") "Undefined" 0 0))
  (bind _output_get (Variables|/Script/Engine.ProjectileMovementComponent|SetInitialSpeed (Variables|/Game/Blueprint/BP_LaserShor.BP_LaserShor_C|GetProjectileMovement _returnvalue) (* (Variables|Default|GetShot_Vel) 1e+02)))
  (bind _output_get_2 (Variables|/Script/Engine.ProjectileMovementComponent|SetMaxSpeed (Variables|/Game/Blueprint/BP_LaserShor.BP_LaserShor_C|GetProjectileMovement _returnvalue) _output_get))
  (Variables|/Script/Engine.MovementComponent|SetVelocity (Variables|/Game/Blueprint/BP_LaserShor.BP_LaserShor_C|GetProjectileMovement _returnvalue) (Math|Vector|MakeVector _output_get_2 0.0 0.0))
  (Variables|Default|SetCharge_shot false))

(fn Barreroll
  (bind _dummy (Variables|Default|Getdummy))
  (bind _relativerotation (Variables|/Script/Engine.SceneComponent|GetRelativeRotation _dummy))
  (Variables|Default|SetVel_mov (Variables|Default|GetVel_mov_barrel))
  (Variables|Default|SetVuelta (+ (Variables|Default|GetBarrel_Vel) (Variables|Default|GetVuelta)))
  (Transformation|SetRelativeRotation _dummy (Math|Rotator|MakeRotator (+ (Variables|Default|GetBarrel_Vel) (.roll _relativerotation)) (.pitch _relativerotation) (.yaw _relativerotation)) false false)
  (if (> (Variables|Default|GetVuelta) 3.6e+02)
    (Variables|Default|SetBarrerrol false)
    (Variables|Default|SetDo_Barreroll 0)
    (Variables|Default|SetVuelta 0.0)
    (Variables|Default|SetVel_mov 2e+02)
    (Transformation|SetRelativeRotation (Variables|Default|Getdummy) "0, 0, 0" false false)))

(fn TimeButtonPress
  (if (Math|Boolean|Equal(Boolean) (Variables|Default|GetX_Press) true)
    (bind _output_get (Variables|Default|SetTime_press_button (+ (Variables|Default|GetTime_press_button) 1)))
    (Development|PrintString (Utilities|String|ToString(Integer) _output_get))))

(fn LoseLife
  (Variables|Default|SetLifes (- (Variables|Default|GetLifes) 1.0))
  (if (== (Variables|Default|GetLifes) 0.0)
    (Game|QuitGame 0 "Quit" false)
    (else
      (Variables|Default|SetHealt 1e+02))))
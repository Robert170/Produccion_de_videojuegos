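; Bomb projectile that damages BP_Adross and ends in a growing explosion.
; On overlap it subtracts Damge from BP_Adross's Life, leaves BP_Enemi unharmed, and waits two seconds for any other actor.
; It then sets the Explotion flag and zeroes projectile velocity.
; While flagged, Tick enlarges the explosion component by a fixed step per frame, destroying the actor at maximum scale.
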(event EventBeginPlay)

(event Collision|EventActorBeginOverlap
  (params (OtherActor :type Actor%20Object%20Reference))
  (Utilities|Casting|CastToBP_Enemi OtherActor
    (:then
      _)
    (:CastFailed
      (bind _asbp_adross (Utilities|Casting|CastToBP_Adross OtherActor)
        (:then
          (Variables|/Game/Blueprint/BP_Adross.BP_Adross_C|SetLife _asbp_adross (- (Variables|/Game/Blueprint/BP_Adross.BP_Adross_C|GetLife _asbp_adross) (Variables|Default|GetDamge))))
        (:CastFailed
          (Utilities|FlowControl|Delay 2.0)))))
  (Variables|Default|SetExplotion%20 true)
  (Variables|/Script/Engine.MovementComponent|SetVelocity (Variables|Default|GetProjectileMovement) "0, 0, 0"))

(event EventTick
  (params (DeltaSeconds :type Float%20%28single-precision%29))
  (if (Math|Boolean|Equal(Boolean) (Variables|Default|GetExplotion%20) true)
    (if (Math|Vector|Equal(Vector) (Variables|Default|GetNew_Sacale) "10.000000,10.000000,10.000000" 0.0001)
      (Actor|DestroyActor)
      (else
        (Variables|Default|SetNew_Sacale (+ (Variables|Default|GetNew_Sacale) "0.100000,0.100000,0.100000"))
        (Transformation|SetRelativeScale3D (Variables|Default|GetExplotion) (Variables|Default|GetNew_Sacale))))))

(fn ConstructionScript)
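; BP_ALLAdross is a multi-part enemy with separate health for its head and two hands, turning to face BP_Arwing actors.
; Overlapping BP_LaserShor actors subtract damage from RightHandLife only, which Tick prints.
; Tick destroys LeftHand or Head when its life runs out, but never the right hand.
; While Head lives, it aims at each Arwing's Dummy, halting if RightHandLife is exactly zero with LeftHand alive.
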(event EventBeginPlay)

(event Collision|EventActorBeginOverlap
  (params (OtherActor :type Actor%20Object%20Reference))
  (bind _asbp_laser_shor (Utilities|Casting|CastToBP_LaserShor OtherActor))
  (Variables|Default|SetRight_Hand_Life (- (Variables|Default|GetRight_Hand_Life) (Variables|/Game/Blueprint/BP_LaserShor.BP_LaserShor_C|GetDamage _asbp_laser_shor))))

(event EventTick
  (params (DeltaSeconds :type Float%20%28single-precision%29))
  (Development|PrintString (Utilities|String|ToString(Float) (Variables|Default|GetRight_Hand_Life)))
  (if (<= (Variables|Default|GetLeft_Hand_Life) 0.0)
    (Components|DestroyComponent (Variables|Default|GetLeft_Hand))
    (if (<= (Variables|Default|GetHead_Life) 0.0) :!label _label
      (Components|DestroyComponent (Variables|Default|GetHead))
      (else
        (bind _outactors (Actor|GetAllActorsOfClass "/Game/Blueprint/BP_Arwing.BP_Arwing_C"))
        (for _array_element _outactors
          (Transformation|SetActorRotation (Math|Rotator|FindLookatRotation (Transformation|GetActorLocation) (Transformation|GetWorldLocation (Variables|/Game/Blueprint/BP_Arwing.BP_Arwing_C|Getdummy _array_element)))))))
    (elif (not (== (Variables|Default|GetRight_Hand_Life) 0.0))
      (goto _label))))

(fn ConstructionScript)
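; BP_Boo is an actor that advances along the Y axis and decides the game's win or lose outcome through overlaps.
; Tick adds Paso to its Y position without delta-time scaling or sweep.
; Reaching BP_FinalBOO stops it and, after a short delay, shows W_WIN.
; Each BP_player overlap decrements NumJu; at zero it shows W_Lose and stops, with both endings switching input to UI-only.
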(event EventBeginPlay
  (Game|Player|SetViewTargetwithBlend (Game|GetPlayerController 0) 0 0.0 "VTBlend_Linear" 0.0 false))

(event Collision|EventActorBeginOverlap
  (params (OtherActor :type Actor%20Object%20Reference))
  (bind _returnvalue (Game|GetPlayerController 0))
  (bind _returnvalue_2 (Game|GetPlayerController 0))
  (Utilities|Casting|CastToBP_FinalBOO OtherActor
    (:then
      (Variables|Default|SetPaso 0.0)
      (Utilities|FlowControl|Delay 0.5)
      (bind _returnvalue_3 (UserInterface|CreateWidget "/Game/Widget/W_WIN.W_WIN_C" _returnvalue))
      (UserInterface|Viewport|AddtoPlayerScreen _returnvalue_3)
      (Variables|/Script/Engine.PlayerController|SetbShowMouseCursor _returnvalue true)
      (Input|SetInputModeUIOnly _returnvalue _returnvalue_3 "DoNotLock"))
    (:CastFailed
      (Utilities|Casting|CastToBP_player OtherActor)
      (Variables|Default|SetNumJu (- (Variables|Default|GetNumJu) 1))
      (if (<= (Variables|Default|GetNumJu) 0)
        (bind _returnvalue_4 (UserInterface|CreateWidget "/Game/Widget/W_Lose.W_Lose_C" _returnvalue_2))
        (UserInterface|Viewport|AddtoPlayerScreen _returnvalue_4)
        (Variables|/Script/Engine.PlayerController|SetbShowMouseCursor _returnvalue_2 false)
        (Input|SetInputModeUIOnly _returnvalue_2 _returnvalue_4 "DoNotLock")
        (Variables|Default|SetPaso 0.0)))))

(event EventTick
  (params (DeltaSeconds :type Float%20%28single-precision%29))
  (bind _returnvalue (Transformation|GetActorLocation))
  (bind (_x _y _z) (Math|Vector|BreakVector _returnvalue))
  (bind _output_get (Variables|Default|Setnew_pos (Math|Vector|MakeVector _x (+ _y (Variables|Default|GetPaso)) _z)))
  (Transformation|SetActorLocation _output_get false false))

(fn ConstructionScript)
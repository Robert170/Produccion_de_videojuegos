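; BP_Plataform3 is a moving platform actor that oscillates vertically every tick.
; Tick advances a phase counter by a step, then offsets the current Z location by the sine of that phase scaled by a limit.
; The offset accumulates on the current position rather than a stored origin, and movement is per frame, without delta time or sweep.
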(event EventBeginPlay)

(event Collision|EventActorBeginOverlap
  (params (OtherActor :type Actor%20Object%20Reference)))

(event EventTick
  (params (DeltaSeconds :type Float%20%28single-precision%29))
  (bind _returnvalue (Transformation|GetActorLocation))
  (bind (_x _y _z) (Math|Vector|BreakVector _returnvalue))
  (Variables|Default|SetPaso%20actual (+ (Variables|Default|GetPaso%20actual) (Variables|Default|GetPaso)))
  (bind _output_get (Variables|Default|SetPos%20Actual (Math|Vector|MakeVector _x _y (+ _z (* (Math|Trig|Sin(Radians) (Variables|Default|GetPaso%20actual)) (Variables|Default|Getlimite))))))
  (Transformation|SetActorLocation _output_get false false))

(fn ConstructionScript)